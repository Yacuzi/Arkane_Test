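; Global game state Blueprint that handles player death restarts and objective notifications.
; On PlayerDied it waits a short delay, then RestartMap reloads the current level by name.
; ObjectiveAdd and ObjectiveComplete each spawn their own UI widget for the first player controller, pass in the objective description and add it to the viewport.
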(event `PlayerDied`
  (`KismetSystemLibrary.Delay` 3.0)
  (`self.RestartMap`))

(fn `ObjectiveAdd`
  (params (ObjectiveDesc :type Text :default "NSLOCTEXT(\"[05E95E8043A463B1FAE08697108D5362]\", \"3EAC83C44531610832772A85A7144399\", \"Bla bla bla bla\")"))
  ;[1 1 1] Displaying new objective
  (bind _returnvalue (`|CreateWidget` "/Game/ArkaneContent/Blueprints/UI/Ark_UI_ObjectiveAdd.Ark_UI_ObjectiveAdd_C" (`GameplayStatics.GetPlayerController` 0)))
  (set `/Game/ArkaneContent/Blueprints/UI/Ark_UI_ObjectiveAdd.ObjectiveDescription` ObjectiveDesc _returnvalue)
  (`UserWidget.AddToViewport` _returnvalue 0))

(fn `ObjectiveComplete`
  (params (ObjectiveDesc :type Text :default "NSLOCTEXT(\"[05E95E8043A463B1FAE08697108D5362]\", \"3EAC83C44531610832772A85A7144399\", \"Bla bla bla bla\")"))
  ;[1 1 1] Displaying completed objective
  (bind _returnvalue (`|CreateWidget` "/Game/ArkaneContent/Blueprints/UI/Ark_UI_ObjectiveComplete.Ark_UI_ObjectiveComplete_C" (`GameplayStatics.GetPlayerController` 0)))
  (set `/Game/ArkaneContent/Blueprints/UI/Ark_UI_ObjectiveComplete.ObjectiveDescription` ObjectiveDesc _returnvalue)
  (`UserWidget.AddToViewport` _returnvalue 0))

(fn `RestartMap`
  (bind _returnvalue (`GameplayStatics.GetCurrentLevelName` true))
  (`GameplayStatics.OpenLevel` (`KismetStringLibrary.Conv_StringToName` _returnvalue)))

(fn `UserConstructionScript`)
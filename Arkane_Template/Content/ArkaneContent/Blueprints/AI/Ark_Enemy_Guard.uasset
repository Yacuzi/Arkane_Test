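; Guard enemy character for the AI, with a gun in its right hand, health, hit reactions and death.
; Attack spawns a beam particle at the gun, and a timeline keeps retracing its endpoint toward the player before destroying it.
; Damage plays a hit montage or, at zero health, triggers Death, which broadcasts, detaches the controller and disables capsule collision.
; Events toggle range-feedback outlines; a temporary debug function prints blackboard state changes.
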(event `self.ReceiveTick`
  (params (DeltaSeconds :type "Float (single-precision)")))

(event `ActivateLaser`
  ;[1 1 1] Laser when aiming at the player
  (bind _returnvalue (`AddComponent|NODE_AddParticleSystemComponent-0` :`bManualAttachment` true))
  (bind _output_get (set `self.BeamParticle` _returnvalue))
  (`ParticleSystemComponent.SetTemplate` _output_get "/Game/ArkaneContent/Effects/ParticleSystems/P_Beam.P_Beam")
  (`SceneComponent.K2_AttachToComponent` (`self.BeamParticle`) (`self.Gun_LaserStart`) "None" "KeepRelative" "KeepRelative" "KeepRelative" true)
  (`Timeline|Laser` :!via `PlayFromStart` :!label _label
    (:`Update`
      (bind _outhit (`KismetSystemLibrary.LineTraceSingle` (`SceneComponent.K2_GetComponentLocation` (`self.BeamParticle`)) (`self.K2_GetActorLocation` (`GameplayStatics.GetPlayerCharacter` 0)) "TraceTypeQuery2"))
      (`ParticleSystemComponent.SetBeamTargetPoint` (`self.BeamParticle`) 0 (`.Location` (`GameplayStatics.BreakHitResult` _outhit)) 0))
    (:`Finished`
      (`ActorComponent.K2_DestroyComponent` (`self.BeamParticle`))
      (set `self.BeamParticle` null))))

(event `StopLaser`
  ;[1 1 1] Laser when aiming at the player
  (goto _label :!via `Stop`))

(event `/Game/ArkaneContent/Blueprints/Ark_DamageInterface.DoDamage`
  (params (DamageAccount :type "Float (single-precision)"))
  ;[1 1 1] Take damage / Hit React / Death
  (bind _output_get (set `self.CurrentHealth` (`KismetMathLibrary.FClamp` (- (`self.CurrentHealth`) DamageAccount) 0.0 (`self.MaxHealth`))))
  (`/Engine/EditorBlueprintResources/StandardMacros.CompareFloat` _output_get
    (:`>`
      (`self.PlayAnimMontage` "/Game/AnimStarterPack/Hit_React_1_Montage.Hit_React_1_Montage")
      (set `self.JustHurt` true))
    (:`==`
      (`self.Death`))))

(event `Show_Outline_OK`
  (`SceneComponent.SetVisibility` (`self.Outline_TooFar`) false false)
  (`SceneComponent.SetVisibility` (`self.Outline_OK`) true false))

(event `Show_Outline_TooFar`
  (`SceneComponent.SetVisibility` (`self.Outline_TooFar`) true false)
  (`SceneComponent.SetVisibility` (`self.Outline_OK`) false false))

(event `Hide_Outlines`
  (`SceneComponent.SetVisibility` (`self.Outline_TooFar`) false false)
  (`SceneComponent.SetVisibility` (`self.Outline_OK`) false false))

(event `Is_Groggy`)

(fn `Attack`
  (`self.ActivateLaser`))

(fn `Death`
  (bind _beamparticle (`self.BeamParticle`))
  (`self.Dead`)
  (`self.DetachFromControllerPendingDestroy`)
  (`PrimitiveComponent.SetCollisionEnabled` (`self.CapsuleComponent`) "NoCollision")
  (`SkeletalMeshComponent.PlayAnimation` (`self.Mesh`) "/Game/AnimStarterPack/Death_1.Death_1" false)
  (if (`KismetSystemLibrary.IsValid` _beamparticle)
    (`ActorComponent.K2_DestroyComponent` _beamparticle)
    (set `self.BeamParticle` null)
    (`self.StopLaser`)))

(fn `GunShot`
  (`AudioComponent.Play` (`self.Audio_Attack`) 0.0))

(fn `Show_State_Bugged`
  (bind _returnvalue (`KismetSystemLibrary.GetObjectName` self))
  ;[1 1 1] TO BE DELETED
  (switch `/Game/ArkaneContent/Blueprints/AI/CustomStructure/Ark_AI_State` (cast `/Game/ArkaneContent/Blueprints/AI/CustomStructure/Ark_AI_State` (`BlackboardComponent.GetValueAsEnum` (`AIBlueprintHelperLibrary.GetBlackboard` self) "State"))
    (:`NewEnumerator0`
      (if (== (`self.State`) 1)
        (set `self.State` 0)
        (`KismetSystemLibrary.PrintString` (`KismetStringLibrary.Concat_StrStr` _returnvalue " Patrol"))))
    (:`NewEnumerator1`
      (if (== (`self.State`) 0)
        (set `self.State` 1)
        (`KismetSystemLibrary.PrintString` (`KismetStringLibrary.Concat_StrStr` _returnvalue " Combat"))))))

(fn `UserConstructionScript`
  (set `self.CurrentHealth` (`self.MaxHealth`))
  (`SceneComponent.K2_AttachToComponent` (`self.Mesh_Gun`) (`self.Mesh`) "hand_r" "KeepRelative" "KeepRelative" "KeepRelative" true))
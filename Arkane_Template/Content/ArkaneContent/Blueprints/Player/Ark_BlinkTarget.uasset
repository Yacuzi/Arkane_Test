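; Blink target actor for the player that shows a marker on the ground beneath its position.
; Each tick it line traces on the Camera channel along its negative up vector, up to a maximum ray distance.
; On a hit, the GroundTarget component is shown and moved slightly above the impact in world Z; otherwise it is hidden.
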(event `self.ReceiveTick`
  (params (DeltaSeconds :type "Float (single-precision)"))
  (bind _returnvalue (`self.K2_GetActorLocation`))
  (bind _groundtarget (`self.GroundTarget`))
  (bind (_outhit _returnvalue_2) (`KismetSystemLibrary.LineTraceSingle` _returnvalue (+ _returnvalue (* (`KismetMathLibrary.NegateVector` (`self.GetActorUpVector`)) (`self.BlinkTargetMaxRayCastDistForGround`))) "TraceTypeQuery2"))
  (if _returnvalue_2
    (`SceneComponent.SetVisibility` _groundtarget true false)
    (`SceneComponent.K2_SetWorldLocation` _groundtarget (+ (`.Location` (`GameplayStatics.BreakHitResult` _outhit)) (0.0 0.0 20.0)) false false)
    (else
      (`SceneComponent.SetVisibility` _groundtarget false false))))

(fn `UserConstructionScript`)
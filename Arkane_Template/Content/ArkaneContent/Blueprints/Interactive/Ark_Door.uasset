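; Interactive sliding door that opens on player interaction or when a non-player actor enters its NPCDetection volume.
; A timeline slides MeshDoor along relative Y, playing to open and reversing to close, with IsOpening tracking the state.
; Interaction toggles the door, but closing is blocked while guards overlap the volume.
; It also closes on end overlap once neither guards nor the player remain inside.
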(event `OpenDoor`
  (set `self.IsOpening` true)
  (bind (_direction _doortranslation) (`Timeline|DoorOpen` :!label _label)
    (:`Update`
      (`SceneComponent.K2_SetRelativeLocation` (`self.Mesh_Door`) (`KismetMathLibrary.MakeVector` 0.0 _doortranslation) false false))))

(event `CloseDoor`
  (set `self.IsOpening` false)
  (goto _label :!via `Reverse`))

(event `self.NPCDetection.OnComponentEndOverlap`
  (params (OverlappedComponent :type "PrimitiveComponent Object Reference") (OtherActor :type "Actor Object Reference") (OtherComp :type "PrimitiveComponent Object Reference") (OtherBodyIndex :type Integer))
  (bind _npcdetection (`self.NPCDetection`))
  ;[1 1 1] Open the door on interaction or when NPC approaches / Closes door on interaction (if no NPC in volume) or when volume is empty
  (if (and (== (`KismetArrayLibrary.Array_Length` (`PrimitiveComponent.GetOverlappingActors` _npcdetection "/Game/ArkaneContent/Blueprints/AI/Ark_Enemy_Guard.Ark_Enemy_Guard_C")) 0) (not (`PrimitiveComponent.IsOverlappingActor` _npcdetection (`GameplayStatics.GetPlayerCharacter` 0))))
    (`self.CloseDoor` :!label _label_2)))

(event `/Game/ArkaneContent/Blueprints/Ark_InteractInterface.Interact`
  ;[1 1 1] Open the door on interaction or when NPC approaches / Closes door on interaction (if no NPC in volume) or when volume is empty
  (if (`self.IsOpening`)
    (if (== (`KismetArrayLibrary.Array_Length` (`PrimitiveComponent.GetOverlappingActors` (`self.NPCDetection`) "/Game/ArkaneContent/Blueprints/AI/Ark_Enemy_Guard.Ark_Enemy_Guard_C")) 0)
      (goto _label_2))
    (else
      (`self.OpenDoor` :!label _label_3))))

(event `self.NPCDetection.OnComponentBeginOverlap`
  (params (OverlappedComponent :type "PrimitiveComponent Object Reference") (OtherActor :type "Actor Object Reference") (OtherComp :type "PrimitiveComponent Object Reference") (OtherBodyIndex :type Integer) (bFromSweep :type Boolean) (SweepResult :type "HitResult Structure (by ref)"))
  ;[1 1 1] Open the door on interaction or when NPC approaches / Closes door on interaction (if no NPC in volume) or when volume is empty
  (if (and (not (`self.IsOpening`)) (!= OtherActor (`GameplayStatics.GetPlayerCharacter` 0)))
    (goto _label_3)))

(fn `UserConstructionScript`)